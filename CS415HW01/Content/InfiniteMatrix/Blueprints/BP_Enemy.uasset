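; BP_Enemy is an enemy actor that damages the player on contact and is destroyed by player contact or projectile hits.
; Overlap events on its Enemy and Hitbox components cast the other actor to BP_Projectile, then to BP_Player, calling HealthDamage on the player.
; Both destroy the enemy on either match, but only the Hitbox handler also destroys the projectile.
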(event OnComponentBeginOverlap(Enemy)
  (params (OverlappedComponent :type Primitive%20Component%20Object%20Reference) (OtherActor :type Actor%20Object%20Reference) (OtherComp :type Primitive%20Component%20Object%20Reference) (OtherBodyIndex :type Integer) (bFromSweep :type Boolean) (SweepResult :type Hit%20Result%20Structure%20%28by%20ref%29))
  (Utilities|Casting|CastToBP_Projectile OtherActor
    (:then
      (Actor|DestroyActor))
    (:CastFailed
      (bind _asbp_player (Utilities|Casting|CastToBP_Player OtherActor))
      (Default|HealthDamage _asbp_player)
      (Actor|DestroyActor))))

(event OnComponentBeginOverlap(hitbox)
  (params (OverlappedComponent :type Primitive%20Component%20Object%20Reference) (OtherActor :type Actor%20Object%20Reference) (OtherComp :type Primitive%20Component%20Object%20Reference) (OtherBodyIndex :type Integer) (bFromSweep :type Boolean) (SweepResult :type Hit%20Result%20Structure%20%28by%20ref%29))
  (bind _asbp_projectile (Utilities|Casting|CastToBP_Projectile OtherActor)
    (:then
      (Actor|DestroyActor)
      (Actor|DestroyActor _asbp_projectile))
    (:CastFailed
      (bind _asbp_player (Utilities|Casting|CastToBP_Player OtherActor))
      (Default|HealthDamage _asbp_player)
      (Actor|DestroyActor))))

(event EventBeginPlay)

(event EventTick
  (params (DeltaSeconds :type Float%20%28single-precision%29)))

(fn ConstructionScript)