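; BP_Projectile is a laser shot that destroys any BP_Enemy it overlaps, then destroys itself.
; Each tick it sweeps along world X at a fixed base speed plus the value returned by the player's SpeedUp function.
; A timer accumulated in Tick destroys the projectile after half a second of flight.
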(event OnComponentBeginOverlap(LaserProjectile)
  (params (OverlappedComponent :type Primitive%20Component%20Object%20Reference) (OtherActor :type Actor%20Object%20Reference) (OtherComp :type Primitive%20Component%20Object%20Reference) (OtherBodyIndex :type Integer) (bFromSweep :type Boolean) (SweepResult :type Hit%20Result%20Structure%20%28by%20ref%29))
  (bind _asbp_enemy (Utilities|Casting|CastToBP_Enemy OtherActor))
  (Utilities|FlowControl|Sequence
    (:then_0
      (Actor|DestroyActor _asbp_enemy))
    (:then_1
      (Actor|DestroyActor))))

(event EventBeginPlay)

(event EventTick
  (params (DeltaSeconds :type Float%20%28single-precision%29))
  (Utilities|FlowControl|Sequence
    (:then_0
      (bind _asbp_player (Utilities|Casting|CastToBP_Player (Game|Player|GetPlayerPawn 0)))
      (bind _newspeed (Default|SpeedUp _asbp_player))
      (Transformation|AddActorWorldOffset (Math|Vector|MakeVector (* (+ _newspeed 4e+03) DeltaSeconds) 0.0 0.0) true))
    (:then_1
      (bind _output_get (Variables|Default|SetTimeElapsed (+ DeltaSeconds (Variables|Default|GetTimeElapsed))))
      (if (>= _output_get 0.5)
        (Actor|DestroyActor)))))

(fn ConstructionScript)